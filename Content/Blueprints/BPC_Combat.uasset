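; Player combat component for BP_ThirdPersonCharacter that handles target lock-on and a sword attack combo.
; The lock input toggles a sphere trace from the camera for pawns, attaches a marker actor to the hit and switches movement to controller-facing rotation.
; Tick aims control rotation at the locked target with a downward pitch offset.
; Attack presses during the montage queue the combo; notifies stop it when none is queued.
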(event `self.ReceiveBeginPlay`
  ; Get Player Class
  (bind _asbp_third_person_character (cast `/Game/ThirdPerson/Blueprints/BP_ThirdPersonCharacter` (`self.GetOwner`)))
  (set `self.Player BP` _asbp_third_person_character))

(event `EnhancedInput|/Game/ThirdPerson/Input/Actions/AI_lock`
  (params (ActionValue :type Boolean) (ElapsedSeconds :type "Float (double-precision)") (TriggeredSeconds :type "Float (double-precision)") (InputAction :type "InputAction Object Reference" :default "/Game/ThirdPerson/Input/Actions/AI_lock.AI_lock"))
  (bind _returnvalue (`Actor.GetTransform` (`self.Target lock Actor`)))
  (bind _transformcomponent (`PlayerCameraManager.TransformComponent` (`GameplayStatics.GetPlayerCameraManager` 0)))
  (bind _charactermovement (`Character.CharacterMovement` (`self.Player BP`)))
  (bind _charactermovement_2 (`Character.CharacterMovement` (`self.Player BP`)))
  (bind (_returnvalue_x _returnvalue_y _returnvalue_z) (`KismetMathLibrary.BreakVector` (`SceneComponent.K2_GetComponentLocation` _transformcomponent)))
  (bind _returnvalue_2 (`KismetMathLibrary.MakeVector` _returnvalue_x _returnvalue_y (+ _returnvalue_z 20.0)))
  ; Target Lock
  (:`Triggered`
    (`self.Target lock Actor`
      (:`then`
        (set `self.Target lock Actor` null)
        (set `CharacterMovementComponent.bOrientRotationToMovement` true _charactermovement)
        (set `CharacterMovementComponent.bUseControllerDesiredRotation` false _charactermovement)
        (`Actor.K2_DestroyActor` (`self.Target lock Widget`)))
      (:`else`
        (bind (_outhit _returnvalue_3) (`KismetSystemLibrary.SphereTraceSingleForObjects` :`Start` _returnvalue_2 :`End` (+ _returnvalue_2 (* (`KismetMathLibrary.GetForwardVector` (`SceneComponent.K2_GetComponentRotation` _transformcomponent)) 1000.0)) :`Radius` 150.0 :`ObjectTypes` (`|MakeArray` "ObjectTypeQuery3" :!type "EObjectTypeQuery Enum") :`DrawDebugType` "ForDuration"))
        (if _returnvalue_3
          (set `self.Target lock Actor` (`.HitActor` (`GameplayStatics.BreakHitResult` _outhit)))
          (set `CharacterMovementComponent.bOrientRotationToMovement` false _charactermovement_2)
          (set `CharacterMovementComponent.bUseControllerDesiredRotation` true _charactermovement_2)
          (bind _returnvalue_4 (`|SpawnActorFromClass` "/Game/Blueprints/BP_TargetLockWidget.BP_TargetLockWidget_C" (`KismetMathLibrary.MakeTransform` (`KismetMathLibrary.MakeVector` (.x (.location _returnvalue)) (.y (.location _returnvalue)) (+ (.z (.location _returnvalue)) 20.0)) (.rotation _returnvalue) (.scale _returnvalue)) "AlwaysSpawn" "MultiplyWithRoot" null null))
          (bind _output_get (set `self.Target lock Widget` _returnvalue_4))
          (`Actor.K2_AttachToActor` _output_get (`self.Target lock Actor`) "None" "SnapToTarget" "SnapToTarget" "SnapToTarget" true))))))

(event `self.ReceiveTick`
  (params (DeltaSeconds :type "Float (single-precision)"))
  (bind (_returnvalue_roll _returnvalue_pitch _returnvalue_yaw) (`KismetMathLibrary.BreakRotator` (`KismetMathLibrary.FindLookAtRotation` (`Actor.K2_GetActorLocation` (`self.Player BP`)) (`Actor.K2_GetActorLocation` (`self.Target lock Actor`)))))
  ; Target Lock
  ;;[0.15 0.02828 0.02828 0.5] Target lock Update
  (`self.Target lock Actor`
    (:`then`
      (`Controller.SetControlRotation` (`Pawn.GetController` (`self.Player BP`)) (`KismetMathLibrary.MakeRotator` _returnvalue_roll (+ _returnvalue_pitch -20.0) _returnvalue_yaw)))
    (:`else`)))

(event `EnhancedInput|/Game/ThirdPerson/Input/Actions/IA_Attack_combo`
  (params (ActionValue :type Boolean) (ElapsedSeconds :type "Float (double-precision)") (TriggeredSeconds :type "Float (double-precision)") (InputAction :type "InputAction Object Reference" :default "/Game/ThirdPerson/Input/Actions/IA_Attack_combo.IA_Attack_combo"))
  (:`Started`
    (if (not (`self.isAttacking?`))
      (set `self.isAttacking?` true)
      (`|PlayMontage` (`Character.Mesh` (`self.Player BP`)) "/Game/Characters/Souls/Combat/SwordAttackCombo_Montage.SwordAttackCombo_Montage"
        (:`OnCompleted`
          (set `self.isAttacking?` false :!label _label)
          (set `self.Combo?` false))
        (:`OnInterrupted`
          (goto _label))
        (:`OnNotifyBegin`
          (if (and (`self.isAttacking?`) (`self.Combo?`))
            (set `self.Combo?` false)
            (else
              (`AnimInstance.Montage_Stop` (`SkeletalMeshComponent.GetAnimInstance` (`Character.Mesh` (`self.Player BP`))) 0.2 "/Game/Characters/Souls/Combat/SwordAttackCombo_Montage.SwordAttackCombo_Montage")
              (set `self.isAttacking?` false)
              (set `self.Combo?` false)))))
      (else
        (set `self.Combo?` true)))))